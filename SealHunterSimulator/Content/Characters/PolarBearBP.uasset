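; Polar bear character Blueprint that varies walk speed with the surface or volume it overlaps and adds sound and particle effects.
; Trigger boxes speed it up, snow piles slow it down, and ending any overlap sets an intermediate speed.
; BeginPlay activates particles and attaches a sound to the mesh, while F plays a voice clip at world origin.
; OnDestroyActor forwards the supplied character to CustomPlayerState.
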(event `self.ReceiveActorBeginOverlap`
  (params (OtherActor :type "Actor Object Reference"))
  (bind _charactermovement (`self.CharacterMovement`))
  (cast `TriggerBox` OtherActor
    (:`then`
      (set `CharacterMovementComponent.MaxWalkSpeed` 500.0 _charactermovement))
    (:`CastFailed`
      (cast `/Game/Landscape/Obstacles/SnowPiles` OtherActor)
      (set `CharacterMovementComponent.MaxWalkSpeed` 200.0 _charactermovement))))

(event `self.ReceiveActorEndOverlap`
  (params (OtherActor :type "Actor Object Reference"))
  (set `CharacterMovementComponent.MaxWalkSpeed` 400.0 (`self.CharacterMovement`)))

(event `Key|F`
  (params (Key :type "Key Structure"))
  (:`Pressed`
    (`GameplayStatics.PlaySoundAtLocation` "/Game/Audio/oh_lord_he_comin.oh_lord_he_comin" (0.0 0.0 0.0) (struct) 1.0 1.0 0.0 null null null)))

(event `self.ReceiveBeginPlay`
  (`ActorComponent.SetActive` (`self.ParticleSystem`) true false)
  (`GameplayStatics.SpawnSoundAttached` "/Game/Audio/PolarBearWump.PolarBearWump" (`self.Mesh`) "None" (0.0 0.0 0.0) (struct) "KeepRelativeOffset" false 1.0 1.0 0.0 null null))

(event `self.onDestroyActor`
  (params (character :type "Actor Object Reference"))
  (bind _ascustom_player_state (cast `/Game/GameStates/CustomPlayerState` (`self.PlayerState`)))
  (`/Game/GameStates/CustomPlayerState.ClientOnActorDestroy` _ascustom_player_state character))

(fn `UserConstructionScript`)